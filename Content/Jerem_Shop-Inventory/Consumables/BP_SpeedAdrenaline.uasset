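; BP_SpeedAdrenaline is a consumable item that temporarily boosts the player's run speed.
; UseItem calls its parent, then adds SpeedForce to the FPS_Character's RunSpeed and reports that the item has a delay.
; A separate DecreaseSpeed event handles the latent wait, subtracting the same amount after Duration and then destroying the item actor.
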(event `DecreaseSpeed`
  (bind _fpscharacter (`self.FPSCharacter`))
  (`KismetSystemLibrary.Delay` (`self.Duration`))
  (set `/Game/FPS_Clovis/Core/PlayerCharacter/FPS_Character.RunSpeed` (- (`/Game/FPS_Clovis/Core/PlayerCharacter/FPS_Character.RunSpeed` _fpscharacter) (`self.SpeedForce`)) _fpscharacter)
  (`self.K2_DestroyActor`))

(fn `UseItem`
  (returns (HasDelay :type Boolean) (Success :type Boolean))
  (locals (IsSuccess :type Boolean :default false))
  (`parent.UseItem`)
  (bind _asfps_character (cast `/Game/FPS_Clovis/Core/PlayerCharacter/FPS_Character` (`GameplayStatics.GetPlayerCharacter` 0)))
  (bind _output_get (set `self.FPSCharacter` _asfps_character))
  ;[1 1 1] Increase speed
  (set `/Game/FPS_Clovis/Core/PlayerCharacter/FPS_Character.RunSpeed` (+ (`/Game/FPS_Clovis/Core/PlayerCharacter/FPS_Character.RunSpeed` _output_get) (`self.SpeedForce`)) _output_get)
  (`self.DecreaseSpeed`)
  (return true (`self.Success`)))

(fn `UserConstructionScript`)