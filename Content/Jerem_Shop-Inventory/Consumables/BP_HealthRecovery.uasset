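; BP_HealthRecovery is a consumable item for the shop and inventory system that restores the player's health.
; Its UseItem override calls the parent logic, then adds RecoverForce to the FPS_Character's CurrentHealth, capped at MaxHealth.
; At full health it prints a message and sets Success to false, and it returns that flag with no delay.
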(fn `UseItem`
  (returns (HasDelay :type Boolean) (Success :type Boolean))
  (locals (FPSCharacter :type "/Game/FPS_Clovis/Core/PlayerCharacter/FPS_Character Object Reference") (IsSuccess :type Boolean :default false))
  (bind _fpscharacter (`local.FPSCharacter`))
  (bind _maxhealth (`/Game/FPS_Clovis/Core/PlayerCharacter/FPS_Character.MaxHealth` _fpscharacter))
  (`parent.UseItem`)
  (bind _asfps_character (cast `/Game/FPS_Clovis/Core/PlayerCharacter/FPS_Character` (`GameplayStatics.GetPlayerCharacter` 0)))
  (bind _output_get (set `local.FPSCharacter` _asfps_character))
  (bind _currenthealth (`/Game/FPS_Clovis/Core/PlayerCharacter/FPS_Character.CurrentHealth` _output_get))
  (if (== _currenthealth _maxhealth)
    (`KismetSystemLibrary.PrintString` "Already full life" true true (struct :`R` 1.0 :`G` 0.259682 :`A` 1.0))
    (set `self.Success` false)
    (else
      (bind _returnvalue (+ _currenthealth (`self.RecoverForce`)))
      (if (<= _returnvalue _maxhealth)
        (set `/Game/FPS_Clovis/Core/PlayerCharacter/FPS_Character.CurrentHealth` _returnvalue _fpscharacter)
        (else
          (set `/Game/FPS_Clovis/Core/PlayerCharacter/FPS_Character.CurrentHealth` _maxhealth _fpscharacter)))))
  (return false (`self.Success`)))

(fn `UserConstructionScript`)