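; BP_Bullet is a projectile actor that damages what it overlaps and pushes physics objects it hits.
; On hit it fires a radial force impulse, then, unless the bullet itself is tagged Player, applies a velocity-scaled impulse to simulating components and destroys itself.
; On overlap it sends damage through BPI_Damageable and destroys itself, ignoring damageable Player-tagged actors and BP_nexus; non-damageable actors simply destroy it.
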(event `self.ReceiveHit`
  (params (MyComp :type "PrimitiveComponent Object Reference") (Other :type "Actor Object Reference") (OtherComp :type "PrimitiveComponent Object Reference") (bSelfMoved :type Boolean) (HitLocation :type "Vector Structure") (HitNormal :type "Vector Structure") (NormalImpulse :type "Vector Structure") (Hit :type "HitResult Structure (by ref)"))
  (`RadialForceComponent.FireImpulse` (`self.RadialForce`))
  (if (not (`self.ActorHasTag` "Player"))
    (if (`SceneComponent.IsSimulatingPhysics` OtherComp "None")
      (`PrimitiveComponent.AddImpulseAtLocation` OtherComp (* (`self.GetVelocity`) (`self.BulletImpulse`)) (`self.K2_GetActorLocation`) "None")
      (`self.K2_DestroyActor`)
      (else
        (`self.K2_DestroyActor`)))))

(event `self.ReceiveActorBeginOverlap`
  (params (OtherActor :type "Actor Object Reference"))
  (if (`KismetSystemLibrary.DoesImplementInterface` OtherActor "/Game/Enemy_Kévin/TopDownShooter/Core/BPI_Damageable.BPI_Damageable_C")
    (if (not (`self.ActorHasTag` OtherActor "Player"))
      (if (!= (`GameplayStatics.GetObjectClass` OtherActor) "/Game/Nexus/BP_nexus.BP_nexus_C")
        (message `/Game/Enemy_Kévin/TopDownShooter/Core/BPI_Damageable.AffectHealth` OtherActor (`self.DammageAmount`))
        (`self.K2_DestroyActor` :!label _label)))
    (else
      (goto _label))))

(fn `UserConstructionScript`)