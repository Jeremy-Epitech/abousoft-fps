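; Master first-person weapon Blueprint that handles raising, firing, aiming down sights and reloading, driven by the WeaponInfo struct.
; Firing loops through a gate for automatic or fires once for semi-auto, using a camera line trace to orient a BP_Bullet carrying damage and impulse.
; Each shot spends ammo, plays effects and montages, and adds random recoil.
; Reloading refills from reserve and blocks aiming, which uses an FOV timeline to zoom.
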(event `self.ReceiveBeginPlay`
  ;[1 1 1] Joue le raise arm quand le joueur sélectionne l'arme pour la prendre en main
  (set `self.CanFire` false)
  (set `self.CanAim` false)
  (`|PlayMontage` (`self.SK_Arms`) (`self.ArmRaiseAnim`)
    (:`OnCompleted`
      (set `self.CanFire` true)
      (set `self.CanAim` true))))

(event `StopAiming`
  ;[1 1 1] Système de visée
  (set `self.isAiming` false :!label _label)
  (bind (_direction _fov) (`Timeline|FOV` :!via `Reverse` :!label _label_2)
    (:`Update`
      (set `CameraComponent.FieldOfView` (`KismetMathLibrary.Lerp` 90.0 50.0 _fov) (`/Game/FPS_Clovis/Core/PlayerCharacter/FPS_Character.FirstPersonCamera` (`self.PlayerRef`))))))

(event `InputAction|Aim`
  (params (Key :type "Key Structure"))
  ;[1 1 1] Système de visée
  (:`Pressed`
    (if (`self.CanAim`)
      (`/Game/FPS_Clovis/Core/PlayerCharacter/FPS_Character.StopSprinting` (`self.PlayerRef`))
      (set `self.isAiming` true)
      (goto _label_2)))
  (:`Released`
    (goto _label)))

(event `StartFiring`
  (bind _playerref (`self.PlayerRef`))
  (bind _sk_weapon (`self.SK_Weapon`))
  (bind _weaponinfo (`self.WeaponInfo`))
  (bind ((`FireRateAutoaticOnly_4_3A325FFF4AD11688FAF7A1A62F6C1F31` _firerateautoaticonly) (`ShootingDistance_6_D8E7AFDE4A67694A7598C788F99BFCE5` _shootingdistance) (`CurrentAmmo_15_15BB892B49344503C8DF03AC07B303C0` _currentammo) (`ShootingType_20_EF57D6D34036201EA34E33B20165A53E` _shootingtype)) (break `/Game/FPS_Clovis/Core/Weapons/Data/S_WeaponInfo` (`self.WeaponInfo`)))
  (bind ((`Damage_2_8DF4A7A04F6678491E03D3B9D27A78A2` _damage) (`BulletImpulse_8_8C10A49E46A1BB6FEAFC7492DBD836DA` _bulletimpulse) (`Recoil_10_BFFB242E4B62F9B1BAB4C59EFA948190` _recoil)) (break `/Game/FPS_Clovis/Core/Weapons/Data/S_WeaponInfo` (`self.WeaponInfo`)))
  (bind _returnvalue (`SceneComponent.GetSocketLocation` (`self.SK_Weapon`) "Fire_FX_Slot"))
  (bind _firstpersoncamera (`/Game/FPS_Clovis/Core/PlayerCharacter/FPS_Character.FirstPersonCamera` (`self.PlayerRef`)))
  (bind _returnvalue_2 (* -1 (`KismetMathLibrary.RandomFloatInRange` 0.0 _recoil)))
  ;[1 1 1] Système de tir
  (`|ExecutionSequence`
    (:`then_0`
      (goto _label_3 :!via `Open`))
    (:`then_1`
      (`/Engine/EditorBlueprintResources/StandardMacros.Gate` true :!label _label_3
        (:`Exit`
          (switch `/Game/FPS_Clovis/Core/Weapons/Data/E_ShootingType` _shootingtype
            (:`NewEnumerator0`
              (`KismetSystemLibrary.RetriggerableDelay` _firerateautoaticonly)
              (`|ExecutionSequence`
                (:`then_0`
                  (goto _label_3))
                (:`then_1`
                  _)))
            (:`NewEnumerator1`
              _))
          (if (<= _currentammo 0)
            (`KismetSystemLibrary.PrintString` "Out of Ammo")
            (`GameplayStatics.PlaySound2D` null 1.0 1.0 0.0 null null)
            (else
              (bind (_outhit _returnvalue_3) (`KismetSystemLibrary.LineTraceSingle` (`SceneComponent.K2_GetComponentLocation` _firstpersoncamera) (+ (* (`SceneComponent.GetForwardVector` _firstpersoncamera) _shootingdistance) (`SceneComponent.GetSocketLocation` (`self.SK_Weapon`) "Fire_FX_Slot")) "TraceTypeQuery1"))
              (if _returnvalue_3
                _
                (else
                  _))
              (bind (_bblockinghit _binitialoverlap _time _distance _location _impactpoint _normal _impactnormal _physmat _hitactor _hitcomponent _hitbonename _hititem _faceindex _tracestart _traceend) (`GameplayStatics.BreakHitResult` _outhit))
              (`GameplayStatics.PlaySoundAtLocation` null _location (struct) 1.0 1.0 0.0 null null null)
              (`GameplayStatics.SpawnEmitterAttached` (`.VFX_23_89EDBD3E4677B87895D288B9369AB573` (break `/Game/FPS_Clovis/Core/Weapons/Data/S_WeaponInfo` (`self.WeaponInfo`))) (`self.SK_Weapon`) "Fire_FX_Slot" (`SceneComponent.GetSocketLocation` _sk_weapon "Fire_FX_Slot") (`SceneComponent.GetSocketRotation` _sk_weapon "Fire_FX_Slot") (1.0 1.0 1.0) "KeepWorldPosition")
              (`|PlayMontage` (`self.SK_Weapon`) (`self.WeaponFireAnim`) ; Pour l'arme
                (:`then`
                  (`|PlayMontage` (`self.SK_Arms`) (select `bool` (`self.isAiming`) :`false` (`self.ArmsFireAnim`) :`true` (`self.ArmsFireAnimADS`)) ; Pour les bras
                    (:`then`
                      (setmembers `/Game/FPS_Clovis/Core/Weapons/Data/S_WeaponInfo` :`StructRef` _weaponinfo :`CurrentAmmo` (- (`.CurrentAmmo_15_15BB892B49344503C8DF03AC07B303C0` (break `/Game/FPS_Clovis/Core/Weapons/Data/S_WeaponInfo` _weaponinfo)) 1))
                      (bind _returnvalue_4 (`|SpawnActorFromClass` "/Game/FPS_Clovis/Core/Weapons/Data/BP_Bullet.BP_Bullet_C" (`KismetMathLibrary.MakeTransform` _returnvalue (`KismetMathLibrary.FindLookAtRotation` _returnvalue (`KismetMathLibrary.SelectVector` _impactpoint _traceend _returnvalue_3))) "Undefined" "OverrideRootScale" null null))
                      (`/Engine/EditorBlueprintResources/StandardMacros.IsValid` _returnvalue_4
                        (:`Is Valid`
                          (set `/Game/FPS_Clovis/Core/Weapons/Data/BP_Bullet.DammageAmount` _damage _returnvalue_4)
                          (set `/Game/FPS_Clovis/Core/Weapons/Data/BP_Bullet.BulletImpulse` _bulletimpulse _returnvalue_4) ; Applique une impulsion sur \nles cibles acteurs touchées
                          (`Pawn.AddControllerPitchInput` _playerref _returnvalue_2)
                          (`Pawn.AddControllerYawInput` _playerref _returnvalue_2))))))))))))))

(event `StopFiring`
  ;[1 1 1] Système de tir
  (goto _label_3 :!via `Close`))

(event `FirePressed`
  ;[1 1 1] Enclenche / Arrête le Système de tir (StartFiring)
  (set `self.CanFire` true)
  (if (not (or (`self.isReloading`) (`/Game/FPS_Clovis/Core/PlayerCharacter/FPS_Character.isSprinting` (`self.PlayerRef`))))
    (`self.StartFiring`)))

(event `FireReleased`
  ;[1 1 1] Enclenche / Arrête le Système de tir (StartFiring)
  (`self.StopFiring`))

(event `Reload`
  (bind ((`ClipSize_13_75C65C704C922CDCC4C0BD932A9B6A7E` _clipsize) (`CurrentAmmo_15_15BB892B49344503C8DF03AC07B303C0` _currentammo)) (break `/Game/FPS_Clovis/Core/Weapons/Data/S_WeaponInfo` (`self.WeaponInfo`)))
  ;[1 1 1] Lance le calcul des munition (WeaponReload) et joue les animations de Reload
  (if (== (`.MaxAmmo_17_0587800D4A3724C1E066E0A8228CC9D1` (break `/Game/FPS_Clovis/Core/Weapons/Data/S_WeaponInfo` (`self.WeaponInfo`))) 0)
    (`KismetSystemLibrary.PrintString` "FIND AMMO")
    (elif (== _clipsize _currentammo)
      (`KismetSystemLibrary.PrintString` "FULL AMMO")
      (else
        (bind _output_get (set `self.isReloading` true))
        (if _output_get
          (set `self.CanFire` false)
          (set `self.CanAim` false)
          (`self.WeaponReload`)
          (`|PlayMontage` (`self.SK_Weapon`) (`self.WeaponReloadAnim`)
            (:`then`
              (`|PlayMontage` (`self.SK_Arms`) (`self.ArmsReloadAnim`)
                (:`OnCompleted`
                  (set `self.isReloading` false)
                  (set `self.CanFire` true)
                  (set `self.CanAim` true))))))))))

(event `WeaponReload`
  (bind _ammoneeded (`self.AmmoNeeded`))
  (bind _weaponinfo (`self.WeaponInfo`))
  (bind ((`MaxAmmo_17_0587800D4A3724C1E066E0A8228CC9D1` _maxammo)) (break `/Game/FPS_Clovis/Core/Weapons/Data/S_WeaponInfo` (`self.WeaponInfo`)))
  (bind ((`ClipSize_13_75C65C704C922CDCC4C0BD932A9B6A7E` _clipsize) (`CurrentAmmo_15_15BB892B49344503C8DF03AC07B303C0` _currentammo)) (break `/Game/FPS_Clovis/Core/Weapons/Data/S_WeaponInfo` (`self.WeaponInfo`)))
  (bind ((`CurrentAmmo_15_15BB892B49344503C8DF03AC07B303C0` _currentammo_2) (`MaxAmmo_17_0587800D4A3724C1E066E0A8228CC9D1` _maxammo_2)) (break `/Game/FPS_Clovis/Core/Weapons/Data/S_WeaponInfo` (`self.WeaponInfo`)))
  ;[1 1 1] Met à jour le nombre de munitions dans le chargeur et le nombre total de munitions
  (if (not (`self.CanFire`))
    (`self.StopAiming`)
    (if (> (`.MaxAmmo_17_0587800D4A3724C1E066E0A8228CC9D1` (break `/Game/FPS_Clovis/Core/Weapons/Data/S_WeaponInfo` (`self.WeaponInfo`))) 0)
      (set `self.AmmoNeeded` (- _clipsize _currentammo))
      (if (<= _maxammo _ammoneeded)
        (setmembers `/Game/FPS_Clovis/Core/Weapons/Data/S_WeaponInfo` :`StructRef` _weaponinfo :`CurrentAmmo` (+ _currentammo_2 _maxammo_2))
        (setmembers `/Game/FPS_Clovis/Core/Weapons/Data/S_WeaponInfo` :`StructRef` _weaponinfo :`MaxAmmo` 0)
        (else
          (setmembers `/Game/FPS_Clovis/Core/Weapons/Data/S_WeaponInfo` :`StructRef` _weaponinfo :`MaxAmmo` (- _maxammo _ammoneeded))
          (setmembers `/Game/FPS_Clovis/Core/Weapons/Data/S_WeaponInfo` :`StructRef` _weaponinfo :`CurrentAmmo` (`.ClipSize_13_75C65C704C922CDCC4C0BD932A9B6A7E` (break `/Game/FPS_Clovis/Core/Weapons/Data/S_WeaponInfo` (`self.WeaponInfo`)))))))))

(fn `CastPlayer`
  (bind _asfps_character (cast `/Game/FPS_Clovis/Core/PlayerCharacter/FPS_Character` (`GameplayStatics.GetPlayerCharacter` 0)))
  (set `self.PlayerRef` _asfps_character))

(fn `UserConstructionScript`
  (`self.CastPlayer`))