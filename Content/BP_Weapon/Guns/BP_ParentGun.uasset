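; BP_ParentGun is a gun actor, named as a parent class, that handles firing and reloading for its parent FirstPersonCharacter.
; FireBullet spawns a BP_Ka74Ammo at the barrel with the camera's rotation, plays sound and an arm montage, and decrements the clip.
; Reload refills the clip from reserve ammo, handling a short reserve.
; StartShooting and StopShooting only toggle IsFiring; nothing here calls FireBullet.
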(event `StartShooting`
  (set `self.IsFiring` true))

(event `StopShooting`
  (set `self.IsFiring` false))

(fn `FireBullet`
  (bind _asfirst_person_character (cast `/Game/FirstPersonBP/Blueprints/FirstPersonCharacter` (`self.GetParentActor`)))
  (if (> (`self.AmmoCurrent`) 0)
    (`|SpawnActorFromClass` "/Game/FPS_Clovis/Core/Weapons/Projectile/BP_Ka74Ammo.BP_Ka74Ammo_C" (`KismetMathLibrary.MakeTransform` (`SceneComponent.K2_GetComponentLocation` (`self.Barrel_Refpoint`)) (`SceneComponent.K2_GetComponentRotation` (`/Game/FirstPersonBP/Blueprints/FirstPersonCharacter.FirstPersonCamera` _asfirst_person_character))) "Undefined" "OverrideRootScale" null null)
    (`GameplayStatics.PlaySoundAtLocation` "/Game/FirstPerson/Audio/FirstPersonTemplateWeaponFire02.FirstPersonTemplateWeaponFire02" (`self.K2_GetActorLocation`) (struct) 0.5 1.0 0.0 null null null) ; Play firing sound
    ;[1 1 1] Animation
    (`AnimInstance.Montage_Play` (`SkeletalMeshComponent.GetAnimInstance` (`/Game/FirstPersonBP/Blueprints/FirstPersonCharacter.Mesh2P` _asfirst_person_character)) "/Game/FirstPerson/Animations/FirstPersonFire_Montage.FirstPersonFire_Montage" 1.0 "MontageLength" 0.0 true)
    (`/Engine/EditorBlueprintResources/StandardMacros.DecrementInt` (`self.AmmoCurrent`))))

(fn `Reload`
  (locals (BulletDiffrence :type Integer))
  ;[1 1 1] Check capacity of recharging
  (bind _output_get (set `local.BulletDiffrence` (- (`self.ClipSize`) (`self.AmmoCurrent`))))
  (if (>= (`self.AmmoMax`) _output_get)
    ;[1 1 1] Set current ammo
    (set `self.AmmoCurrent` (`self.ClipSize`))
    ;[1 1 1] Set Ammo max
    (set `self.AmmoMax` (- (`self.AmmoMax`) (`local.BulletDiffrence`)))
    (else
      (set `self.AmmoCurrent` (+ (`self.AmmoCurrent`) (`self.AmmoMax`)))
      (set `self.AmmoMax` 0))))

(fn `UserConstructionScript`)