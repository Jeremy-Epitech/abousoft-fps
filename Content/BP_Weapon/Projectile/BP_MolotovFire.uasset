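; Molotov fire area actor that repeatedly damages actors standing in it and expires after a short lifespan.
; On BeginPlay it reads its damage from the player character's MolotovThrown data and starts the damage loop.
; Overlaps on the Rr component maintain a target array, and a gated, self-calling Delay loop damages those implementing BPI_Damageable each second.
; The fire sound call is disconnected.
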(event `self.ReceiveBeginPlay`
  (bind _asfps_character (cast `/Game/FPS_Clovis/Core/PlayerCharacter/FPS_Character` (`GameplayStatics.GetPlayerCharacter` 0)))
  (bind _output_get (set `self.FPSCharacter` _asfps_character))
  (bind _result (`/Engine/EditorBlueprintResources/StandardMacros.NegateFloat` (`/Game/BP_Weapon/Projectile/BP_Molotov.Dammage` (`/Game/FPS_Clovis/Core/PlayerCharacter/FPS_Character.MolotovThrown` _output_get)))
    (:`  `
      (set `self.Dammage` _result)
      (`self.StartDammage`)
      (`self.SetLifeSpan` 7.0))))

(event `self.ReceiveTick`
  (params (DeltaSeconds :type "Float (single-precision)")))

(event `ContinueDammage`
  ;[1 1 1] Affect health
  (`/Engine/EditorBlueprintResources/StandardMacros.Gate` true :!label _label
    (:`Exit`
      (for _array_element (`self.TargetArray`)
        (if (`KismetSystemLibrary.DoesImplementInterface` _array_element "/Game/Enemy_Kévin/TopDownShooter/Core/BPI_Damageable.BPI_Damageable_C")
          (message `/Game/Enemy_Kévin/TopDownShooter/Core/BPI_Damageable.AffectHealth` _array_element (`self.Dammage`))))
      (`KismetSystemLibrary.Delay` 1.0)
      (`self.ContinueDammage`))))

(event `StartDammage`
  ;[1 1 1] Affect health
  (`|ExecutionSequence`
    (:`then_0`
      (goto _label :!via `Open`))
    (:`then_1`
      (goto _label))))

(event `StopDammage`
  ;[1 1 1] Affect health
  (goto _label :!via `Close`))

(event `self.rr.OnComponentBeginOverlap`
  (params (OverlappedComponent :type "PrimitiveComponent Object Reference") (OtherActor :type "Actor Object Reference") (OtherComp :type "PrimitiveComponent Object Reference") (OtherBodyIndex :type Integer) (bFromSweep :type Boolean) (SweepResult :type "HitResult Structure (by ref)"))
  ;[1 1 1] Overlap detection
  (`/Engine/EditorBlueprintResources/StandardMacros.IsValid` OtherActor
    (:`Is Valid`
      (`KismetArrayLibrary.Array_Add` (`self.TargetArray`) OtherActor))))

(event `self.rr.OnComponentEndOverlap`
  (params (OverlappedComponent :type "PrimitiveComponent Object Reference") (OtherActor :type "Actor Object Reference") (OtherComp :type "PrimitiveComponent Object Reference") (OtherBodyIndex :type Integer))
  (bind _targetarray (`self.TargetArray`))
  ;[1 1 1] Overlap detection
  (`/Engine/EditorBlueprintResources/StandardMacros.IsValid` OtherActor
    (:`Is Valid`
      (if (`KismetArrayLibrary.Array_Contains` _targetarray OtherActor)
        (`KismetArrayLibrary.Array_RemoveItem` _targetarray OtherActor)))))

(fn `UserConstructionScript`)